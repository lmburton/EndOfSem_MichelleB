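; BP_ElevatorPlatform is an elevator platform that travels vertically between its start position and a fixed point above it.
; BeginPlay caches both endpoints from the actor's location.
; CallElevator plays or reverses the MoveElevator timeline based on IsUp, lerping the actor between the endpoints without sweep.
; IsUp flips when the timeline finishes.
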(event `self.ReceiveBeginPlay`
  (bind _output_get (set `self.StartLocation` (`self.K2_GetActorLocation`)))
  (bind _output_get_2 (set `self.EndLocation` (+ (`self.K2_GetActorLocation`) (0.0 0.0 890.0)))))

(event `CallElevator`
  (if (`self.IsUp`)
    (bind (_direction _alpha) (`Timeline|MoveElevator` :!via `Reverse` :!label _label)
      (:`Update`
        (`self.K2_SetActorLocation` (`KismetMathLibrary.VLerp` (stale `self.ReceiveBeginPlay` _output_get) (stale `self.ReceiveBeginPlay` _output_get_2) _alpha)))
      (:`Finished`
        (set `self.IsUp` (not (`self.IsUp`)))))
    (else
      (goto _label))))

(fn `UserConstructionScript`)